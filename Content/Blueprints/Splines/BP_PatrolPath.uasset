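; BP_PatrolPath is a spline-based enemy patrol route that tracks a current point and exposes its world location.
; EvaluateCurrentPathPoint steps the index by Direction, ping-ponging by reversing when it runs past either end of EnemyRouteSpline.
; On reversal it steps back onto the endpoint, so that point repeats, and raises IsEndOfPath until the next evaluation, readable through IsPathEnd.
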(event `EvaluateCurrentPathPoint`
  ;[0 0 0 0] Logic to increment/decrement patrol path points(spline)
  (if (`self.IsEndOfPath`)
    (set `self.IsEndOfPath` false))
  (`self.IncrementPatrolPoint`)
  (if (== (`self.CurrentPathPoint`) (`SplineComponent.GetNumberOfSplinePoints` (`self.EnemyRouteSpline`)))
    (set `self.Direction` -1)
    (set `self.IsEndOfPath` true)
    (`self.IncrementPatrolPoint`)
    (elif (== (`self.CurrentPathPoint`) -1)
      (set `self.Direction` 1)
      (set `self.IsEndOfPath` true)
      (`self.IncrementPatrolPoint`))))

(fn `GetPathPointWorldLocation`
  (returns (SplinePointLocation :type "Vector Structure"))
  ;[0 0 0 0] Function to get world location of the patrol points
  (return (`SplineComponent.GetLocationAtSplinePoint` (`self.EnemyRouteSpline`) (`self.CurrentPathPoint`) "World")))

(fn `IncrementPatrolPoint`
  ;[0 0 0 0] Function to increment patrol points
  (set `self.CurrentPathPoint` (+ (`self.CurrentPathPoint`) (`self.Direction`))))

(fn `IsPathEnd`
  (returns (PathEnded :type Boolean))
  (return (`self.IsEndOfPath`)))

(fn `UserConstructionScript`)