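; AI controller that moves an enemy pawn around a looping patrol route defined by a spline.
; On possess it gets the patrol path from the pawn through GetPatrolPathMessage and caches the spline point count.
; FollowPatrolPath moves to the current point, and each successful move advances the index, resets it past the count and repeats.
; The patrol loop is not started within this graph.
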(event `self.ReceivePossess`
  (params (PossessedPawn :type "Pawn Object Reference"))
  (bind _output_get (set `self.EnemyPawn` PossessedPawn))
  (bind _enemypath (message `/Game/Blueprints/Interfaces/BPI_EnemyPatrol.GetPatrolPath` _output_get))
  (bind _output_get_2 (set `self.EnemyPatrolPath` _enemypath))
  (set `self.MaxPatrolPoints` (`SplineComponent.GetNumberOfSplinePoints` (`/Game/Blueprints/Splines/BP_PatrolPath.EnemyRouteSpline` _output_get_2))))

(event `/Game/Blueprints/Interfaces/BPI_EnemyController.FollowPatrolPath`
  (`|AIMoveTo` (`self.EnemyPawn`) (`SplineComponent.GetLocationAtSplinePoint` (`/Game/Blueprints/Splines/BP_PatrolPath.EnemyRouteSpline` (`self.EnemyPatrolPath`)) (`self.CurrentPatrolPoints`) "World") null
    (:`OnSuccess`
      (`self.FindNextPatrolPoint`))))

(event `FindNextPatrolPoint`
  (bind _result (`/Engine/EditorBlueprintResources/StandardMacros.IncrementInt` (`self.CurrentPatrolPoints`))
    (:`  `
      (if (> _result (`self.MaxPatrolPoints`))
        (set `self.CurrentPatrolPoints` 0))
      (`self.FollowPatrolPath`))))

(fn `UserConstructionScript`)