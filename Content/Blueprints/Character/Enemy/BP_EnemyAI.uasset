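; Enemy AI character Blueprint exposing interface events and queries for movement, facing, health and patrol path.
; Movement events override walk speed or restore a saved default; turning stops movement and snaps yaw toward a stimulus location.
; Health events apply damage or healing without clamping, alongside threshold and max-health checks.
; Attack is a placeholder that prints a message and immediately calls AttackFinished.
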(event `/Game/Blueprints/Interfaces/BPI_EnemyPatrol.SaveDefaultMovementSpeed`
  ;[0 0 0 0] Save Default Movement Speed
  (set `self.Max Walk Speed` (`CharacterMovementComponent.MaxWalkSpeed` (`self.CharacterMovement`))))

(event `/Game/Blueprints/Interfaces/BPI_EnemyPatrol.SetMovementSpeed`
  (params (EnemyMovementSpeed :type "Float (double-precision)"))
  ;[0 0 0 0] Interface Event to Set Movement Speed
  (set `CharacterMovementComponent.MaxWalkSpeed` EnemyMovementSpeed (`self.CharacterMovement`)))

(event `/Game/Blueprints/Interfaces/BPI_EnemyPatrol.SetDefaultMovementSpeed`
  ;[0 0 0 0] Interface Event to Set Default Movement Speed
  (set `CharacterMovementComponent.MaxWalkSpeed` (`self.Max Walk Speed`) (`self.CharacterMovement`)))

(event `/Game/Blueprints/Interfaces/BPI_EnemyPatrol.TurnEnemyTowardsStimulus`
  (params (StimulusLocation :type "Vector Structure"))
  (bind (_returnvalue_roll _returnvalue_pitch) (`KismetMathLibrary.BreakRotator` (`self.K2_GetActorRotation`)))
  (bind (_returnvalue_roll_2 _returnvalue_pitch_2 _returnvalue_yaw) (`KismetMathLibrary.BreakRotator` (`KismetMathLibrary.FindLookAtRotation` (`self.K2_GetActorLocation`) StimulusLocation)))
  ;[0 0 0 0] Interface Event to Rotate Enemy towards Player
  (`MovementComponent.StopMovementImmediately` (`self.CharacterMovement`))
  (`self.K2_SetActorRotation` (`KismetMathLibrary.MakeRotator` _returnvalue_roll _returnvalue_pitch _returnvalue_yaw))
  (`CharacterMovementComponent.SetMovementMode` (`self.CharacterMovement`) "MOVE_Walking" 0))

(event `Attack`
  ;[0 0 0 0] Custom Event - Any attack logic(anim) can be added here
  (`KismetSystemLibrary.PrintString` "Enemy Attack Player!")
  (`self.AttackFinished`))

(event `/Game/Blueprints/Interfaces/BPI_EnemyInteract.HealthHit`
  (params (HealthDamage :type "Float (double-precision)"))
  ;[0 0 0 0] Interface Event - Logic to reduce health when hit
  (bind _output_get (set `self.Health` (- (`self.Health`) HealthDamage)))
  (`KismetSystemLibrary.PrintString` (`KismetStringLibrary.Conv_DoubleToString` _output_get) true true (struct :`G` 0.66 :`B` 1.0 :`A` 1.0) 2.0 "None"))

(event `/Game/Blueprints/Interfaces/BPI_EnemyInteract.AddHealth`
  (params (HealthAmountAdded :type "Float (double-precision)"))
  ;[0 0 0 0] Interface Event - Logic to add health when healed
  (bind _output_get (set `self.Health` (+ HealthAmountAdded (`self.Health`))))
  (`KismetSystemLibrary.PrintString` (`KismetStringLibrary.Conv_DoubleToString` _output_get) true true (struct :`G` 0.66 :`B` 1.0 :`A` 1.0) 2.0 "None"))

(fn `GetPatrolPath`
  (returns (EnemyPath :type "/Game/Blueprints/Splines/BP_PatrolPath Object Reference"))
  (return (`self.AIPatrolPath`)))

(fn `HasHealthReachedThreshold`
  (params (HealthThreshold :type "Float (double-precision)"))
  (returns (HealthRecovered :type Boolean))
  (return (< HealthThreshold (`self.Health`))))

(fn `IsHealthBelowThreshold`
  (params (HealthThreshold :type "Float (double-precision)"))
  (returns (CriticalHealth :type Boolean))
  (return (< (`self.Health`) HealthThreshold)))

(fn `IsMaxHealthReached`
  (returns (MaxHealthReached :type Boolean))
  (return (>= (`self.Health`) (`self.MaxHealth`))))

(fn `UserConstructionScript`)